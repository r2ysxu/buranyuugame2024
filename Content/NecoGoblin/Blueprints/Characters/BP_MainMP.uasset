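; Player character Blueprint that adds camera-distance material updates and Escape-key menu handling.
; On BeginPlay and whenever camera distance changes, it writes the distance to the CameraLocation_MatParam material parameter collection so materials can read it.
; Escape calls OnShowSkills on the player's MainMPCharacter if the skill menu is open.
; Otherwise it opens HUD_PauseMenu, pauses the game and switches to focused, UI-only input with a cursor.
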(event EventBeginPlay
  (bind _returnvalue (Class|MainCharacter|GetCameraDistance))
  (Rendering|Material|SetScalarParameterValue "/Game/NecoGoblin/VFX/CameraLocation_MatParam.CameraLocation_MatParam" "Distance" _returnvalue :!class /Script/Engine.KismetMaterialLibrary))

(event Collision|EventActorBeginOverlap
  (params (OtherActor :type Actor%20Object%20Reference)))

(event EventTick
  (params (DeltaSeconds :type Float%20%28single-precision%29)))

(event EventOnCameraDistanceChanged
  (bind _returnvalue (Class|MainCharacter|GetCameraDistance))
  (Rendering|Material|SetScalarParameterValue "/Game/NecoGoblin/VFX/CameraLocation_MatParam.CameraLocation_MatParam" "Distance" _returnvalue :!class /Script/Engine.KismetMaterialLibrary))

(event Input|KeyboardEvents|Escape
  (params (Key :type Key%20Structure :default "None"))
  (bind _returnvalue (Game|GetPlayerController 0))
  (:Pressed
    (bind _asmain_mpcharacter (Utilities|Casting|CastToMainMPCharacter (Game|GetPlayerCharacter 0)))
    (bind _returnvalue_2 (Class|MainCharacter|GetIsSkillMenuOpen _asmain_mpcharacter))
    (if _returnvalue_2
      (Class|MainCharacter|OnShowSkills _asmain_mpcharacter)
      (else
        (bind _returnvalue_3 (UserInterface|CreateWidget "/Game/NecoGoblin/HUD/MenuUI/HUD_PauseMenu.HUD_PauseMenu_C" _returnvalue))
        (UserInterface|Viewport|AddtoViewport _returnvalue_3 0)
        (Variables|/Script/Engine.PlayerController|SetbShowMouseCursor _returnvalue true)
        (Game|SetGamePaused true)
        (Input|SetInputModeUIOnly _returnvalue _returnvalue_3 "DoNotLock" false)
        (Widget|SetKeyboardFocus _returnvalue_3)))))

(fn ConstructionScript)