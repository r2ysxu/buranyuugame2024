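; Game mode for NecoGoblin that handles the opening main menu and the victory outro.
; On BeginPlay it adds the main menu HUD, shows the cursor, pauses the game and switches input to UI only.
; OnVictoryAchieved teleports the possessed MainCharacter to a hardcoded location, disables player input and plays the OutroScene level sequence.
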(event EventBeginPlay
  (bind _returnvalue (Game|GetPlayerController 0))
  (bind _returnvalue_2 (UserInterface|CreateWidget "/Game/NecoGoblin/HUD/MenuUI/HUD_MainMenu.HUD_MainMenu_C" _returnvalue))
  (UserInterface|Viewport|AddtoViewport _returnvalue_2 0)
  (Variables|/Script/Engine.PlayerController|SetbShowMouseCursor _returnvalue true)
  (Game|SetGamePaused true)
  (Input|SetInputModeUIOnly _returnvalue _returnvalue_2 "DoNotLock" false))

(event EventTick
  (params (DeltaSeconds :type Float%20%28single-precision%29)))

(event EventOnVictoryAchieved
  (bind _returnvalue (Game|GetPlayerController 0))
  (bind _asmain_character (Utilities|Casting|CastToMainCharacter (Pawn|GetControlledPawn _returnvalue)))
  (Transformation|SetActorLocation _asmain_character "11104.353395,10520.240213,2858.843941" false true)
  (Input|DisableInput _returnvalue)
  (bind _returnvalue_2 (Sequencer|Player|CreateLevelSequencePlayer "/Game/NecoGoblin/Cine/OutroScene.OutroScene"))
  (Sequencer|Player|Play _returnvalue_2 :!class /Script/MovieScene.MovieSceneSequencePlayer))

(fn ConstructionScript)