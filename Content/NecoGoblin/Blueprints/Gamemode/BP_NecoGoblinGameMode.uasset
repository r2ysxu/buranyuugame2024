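; Game mode for NecoGoblin that handles the start menu and the victory outro.
; On BeginPlay it shows the single-player start menu, starts its music, shows the mouse cursor and pauses the game.
; On victory it teleports the MainCharacter to a fixed spot, disables input, plays the OutroScene sequence, then reopens IslandMap after a short delay.
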(event EventBeginPlay
  (bind _returnvalue (Game|GetPlayerController 0))
  (bind _returnvalue_2 (UserInterface|CreateWidget "/Game/NecoGoblin/Menus/Menu_StartSPMain.Menu_StartSPMain_C" _returnvalue))
  (UserInterface|Viewport|AddtoViewport _returnvalue_2 0)
  (Default|PlayMusic _returnvalue_2)
  (Variables|/Script/Engine.PlayerController|SetbShowMouseCursor _returnvalue true)
  (Game|SetGamePaused true))

(event EventTick
  (params (DeltaSeconds :type Float%20%28single-precision%29)))

(event EventOnVictoryAchieved
  (bind _returnvalue (Game|GetPlayerController 0))
  (bind _returnvalue_2 (Pawn|GetControlledPawn _returnvalue))
  (bind _asmain_character (Utilities|Casting|CastToMainCharacter _returnvalue_2))
  (Transformation|SetActorLocation _asmain_character "11104.353395,10520.240213,2858.843941" false true)
  (Input|DisableInput _returnvalue_2 0)
  (bind _returnvalue_3 (Sequencer|Player|CreateLevelSequencePlayer "/Game/NecoGoblin/Cine/OutroScene.OutroScene"))
  (Sequencer|Player|Play _returnvalue_3 :!class /Script/MovieScene.MovieSceneSequencePlayer)
  (Utilities|FlowControl|Delay 5.0)
  (Game|OpenLevel(byObjectReference) "/Game/NecoGoblin/Maps/IslandMap.IslandMap"))

(fn ConstructionScript)